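; BP_Actor is an actor that reports its stats on screen and moves continuously.
; On BeginPlay it prints its name, health and defense variables (Nombre, Vida, Defensa) as one message in a configurable color.
; Every Tick it applies a local offset and rotation from variables, plus a fixed world-space drift along X.
; Movement is applied per frame without delta-time scaling or sweep, so speed depends on frame rate.
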(event EventBeginPlay
  (Development|PrintString (Utilities|String|Append "Nombre:" (Variables|Propiedades|GetNombre) " 
VIda:" (Utilities|String|ToString(Integer) (Variables|Propiedades|GetVida)) " 
Defensa:" (Utilities|String|ToString(Float) (Variables|Propiedades|GetDefensa))) true true (Variables|Propiedades|GetColorMensaje) 3e+01))

(event EventTick
  (params (DeltaSeconds :type Float%20%28single-precision%29))
  (Transformation|AddActorLocalOffset (Variables|Propiedades|GetVelocidad) false false)
  (Transformation|AddActorLocalRotation (Variables|Propiedades|GetVelocidadRotacion) false false)
  (Transformation|AddActorWorldOffset "5.000000,0.000000,0.000000"))

(fn ConstructionScript)